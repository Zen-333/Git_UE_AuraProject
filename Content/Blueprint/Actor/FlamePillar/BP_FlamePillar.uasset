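; BP_FlamePillar is a flame pillar actor whose FireLight flickers in intensity.
; From BeginPlay, it randomly picks one of two intensity timelines and plays it from the start, then picks again whenever one finishes.
; Each timeline update feeds ScaleFlameIntensity, which multiplies the curve value by BaseIntensity and applies it to the light, so the flicker needs no Tick.
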(event Custom|StartTimeLine_1
  (bind _light_intensity (Timeline|FlameIntensity_1 PlayFromStart)
    (:Update
      (CallFunction|ScaleFlameIntensity _light_intensity))
    (:Finished
      (CallFunction|ChooseTimeLine))))

(event Custom|StartTimeLine_2
  (bind _lightintensity (Timeline|FlameIntensity_2 PlayFromStart)
    (:Update
      (CallFunction|ScaleFlameIntensity _lightintensity))
    (:Finished
      (CallFunction|ChooseTimeLine))))

(event Custom|ChooseTimeLine
  (switch int (Math|Random|RandomIntegerinRange 0 1)
    (:Default
      (CallFunction|StartTimeLine2 :!label _label))
    (:0
      (CallFunction|StartTimeLine1))
    (:1
      (goto _label))))

(event EventBeginPlay
  (CallFunction|ChooseTimeLine))

(event Collision|EventActorBeginOverlap
  (params (OtherActor :type Actor%20Object%20Reference)))

(event EventTick
  (params (DeltaSeconds :type Float%20%28single-precision%29)))

(fn ConstructionScript)

(fn ScaleFlameIntensity
  (params (Intensity :type Float%20%28double-precision%29))
  (Rendering|Components|Light|SetIntensity (Variables|Default|GetFireLight) (* Intensity (Variables|Default|GetBase%20Intensity))))