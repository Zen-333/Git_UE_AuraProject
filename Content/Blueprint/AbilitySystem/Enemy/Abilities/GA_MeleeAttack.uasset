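; Enemy melee attack Gameplay Ability that turns the avatar toward its combat target and plays a random tagged attack montage.
; When the montage's gameplay event arrives, it finds live players in a small sphere at that montage's combat socket and applies damage to non-friends.
; A hit fires one MeleeImpact gameplay cue tagged with the montage tag.
; The ability ends after that event or when the montage completes or is interrupted.
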(event Ability|EventActivateAbility
  (bind _returnvalue (Ability|GetAvatarActorfromActorInfo))
  (bind _returnvalue_2 (Ability|GetAvatarActorfromActorInfo))
  (Variables|Default|SetHasHitTarget false)
  (bind _returnvalue_3 (Class|EnemyInterface|GetCombatTarget(Message) _returnvalue_2))
  (bind _ascombat_interface (Utilities|Casting|CastToCombatInterface _returnvalue_2))
  (Class|CombatInterface|UpdateFacingTarget _ascombat_interface (Transformation|GetActorLocation _returnvalue_3))
  (bind _returnvalue_4 (Class|CombatInterface|GetAttackMontages(Message) (Ability|GetAvatarActorfromActorInfo)))
  (bind _output_get (Variables|Default|SetTagged%20Montage (Class|AuraDamageGameplayAbility|GetRandomTaggedMontagefromArray _returnvalue_4)))
  (|PlayMontageandWaitProxy "None" (.montage _output_get) 1.0 "None" false 1.0 0.0
    (:then
      (Ability|Tasks|WaitGameplayEvent (.montagetag _output_get) 0
        (:EventReceived
          (bind _returnvalue_5 (Class|CombatInterface|GetCombatSocketLocation(Message) _returnvalue (.SocketTag (Utilities|Struct|BreakTaggedMontage (Variables|Default|GetTagged%20Montage)))))
          (bind _output_get_2 (Variables|Default|SetCombatSocketLocation _returnvalue_5))
          (bind _outoverlapingactors (Class|AuraAbilitySystemLibrary|GetLivePlayerWithinRadius _returnvalue (Utilities|Array|MakeArray _returnvalue) 45.0 _output_get_2))
          (for _array_element _outoverlapingactors
            (if (Class|AuraAbilitySystemLibrary|IsNotFirend (Ability|GetAvatarActorfromActorInfo) _array_element)
              (Class|AuraAbilitySystemLibrary|ApplyDamageEffect (Class|AuraDamageGameplayAbility|MakeDamageEffectParamsfromClassDefaults _array_element))
              (Variables|Default|SetHasHitTarget true)))
          (if (Variables|Default|GetHasHitTarget)
            (bind _returnvalue_6 (Class|EnemyInterface|GetCombatTarget(Message) (Ability|GetAvatarActorfromActorInfo)))
            (Class|GameplayAbility|ExecuteGameplayCuewithParams "(TagName=\"GameplayCue.MeleeImpact\")" (Ability|GameplayCue|MakeGameplayCueParameters :AggregatedSourceTags (GameplayTags|MakeGameplayTagContainerfromTag (.MontageTag (Utilities|Struct|BreakTaggedMontage (Variables|Default|GetTagged%20Montage)))) :Location (Variables|Default|GetCombatSocketLocation) :EffectCauser (Ability|GetAvatarActorfromActorInfo) :SourceObject _returnvalue_6)))
          (Ability|EndAbility))))
    (:OnCompleted
      (Ability|EndAbility :!label _label))
    (:OnInterrupted
      (goto _label))
    (:OnCancelled
      (goto _label))))

(event Ability|EventOnEndAbility
  (params (bWasCancelled :type Boolean)))