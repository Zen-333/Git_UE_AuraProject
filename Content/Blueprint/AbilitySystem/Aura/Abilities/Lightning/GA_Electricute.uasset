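; Gameplay ability for Electricute, a held lightning beam fired toward the target under the mouse.
; It hides the cursor, faces the target and plays a montage, whose event disables movement and starts the beam.
; ShockLoop gameplay cues render the beam from weapon to first target, chaining to additional targets if that target implements CombatInterface.
; Input release restores cursor and movement, removes cues using stored parameters and ends the ability.
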(event Ability|EventActivateAbility
  (CallFunction|EnforceImplementsCombatInterface)
  (bind _datahandle (|TargetDataUnderMouse)
    (:ValidData
      (Class|AuraBeemSpell|StoreMouseDataInfo (Ability|TargetData|GetHitResultfromTargetData _datahandle))
      (Class|AuraBeemSpell|StoreOwnerVariables)
      (Utilities|FlowControl|Sequence
        (:then_0
          (Variables|/Script/Engine.PlayerController|SetbShowMouseCursor (Variables|Default|GetOwnerPlayerController) false)
          (CallFunction|UpdateFacingTarget)
          (GameplayCue|ExecuteGameplayCue :GameplayCueTag "(TagName=\"GameplayCue.ShockBurst\")")
          (|PlayMontageandWaitProxy "None" (Variables|Default|GetMontageElectricute) 1.0 "None" false 1.0 0.0
            (:then
              (Ability|Tasks|WaitGameplayEvent "(TagName=\"Event.Montage.Electricute\")" 0 true
                (:EventReceived
                  (CallFunction|InShockLoop)
                  (CallFunction|SpawnElecticBeam))))))
        (:then_1
          (Ability|Tasks|WaitInputRelease false
            (:OnRelease
              (CallFunction|PreparetoEndAbility)
              (Ability|EndAbility))))))))

(fn EnforceImplementsCombatInterface
  (if (not (Utilities|DoesObjectImplementInterface (Ability|GetAvatarActorfromActorInfo) "/Script/Aura.CombatInterface"))
    (Ability|EndAbility)))

(fn PreparetoEndAbility
  (Variables|/Script/Engine.PlayerController|SetbShowMouseCursor (Variables|Default|GetOwnerPlayerController) true)
  (Class|CombatInterface|SetinShockLoop(Message) (Ability|GetAvatarActorfromActorInfo) false)
  (Pawn|Components|CharacterMovement|SetMovementMode (Variables|/Script/Engine.Character|GetCharacterMovement (Variables|Default|GetOwningCharacter)) "MOVE_Walking" 0)
  (if (Variables|Default|GetFirstTargetImplementsInterface)
    (GameplayCue|RemoveGameplayCueOnActor(Looping) (Variables|Default|GetMouseHitActor) "(TagName=\"GameplayCue.ShockLoop\")" (Variables|Default|GetFirstTargetCueParams))
    (for _array_element (Variables|Default|GetAdditional%20Targets)
      (CallFunction|RemoveShockLoopfromAdditionalTargets _array_element))
    (else
      (GameplayCue|RemoveGameplayCueOnActor(Looping) (Ability|GetAvatarActorfromActorInfo) "(TagName=\"GameplayCue.ShockLoop\")" (Variables|Default|GetFirstTargetCueParams)))))

(fn InShockLoop
  (Class|CombatInterface|SetinShockLoop(Message) (Ability|GetAvatarActorfromActorInfo) true)
  (Pawn|Components|CharacterMovement|DisableMovement (Variables|/Script/Engine.Character|GetCharacterMovement (Variables|Default|GetOwningCharacter))))

(fn UpdateFacingTarget
  (Class|CombatInterface|UpdateFacingTarget(Message) (Ability|GetAvatarActorfromActorInfo) (Variables|Default|GetMouseHitLocation)))

(fn SpawnElecticBeam
  (Class|AuraBeemSpell|TraceFirstTarget (Variables|Default|GetMouseHitLocation))
  (bind _returnvalue (Class|CombatInterface|GetWeapon(Message) (Variables|Default|GetOwningCharacter)))
  (Variables|Default|SetFirstTargetCueParams (Ability|GameplayCue|MakeGameplayCueParameters :Location (Variables|Default|GetMouseHitLocation) :SourceObject (Variables|Default|GetMouseHitActor) :TargetAttachComponent _returnvalue))
  (bind _output_get (Variables|Default|SetFirstTargetImplementsInterface (Utilities|DoesObjectImplementInterface (Variables|Default|GetMouseHitActor) "/Script/Aura.CombatInterface")))
  (if _output_get
    (Variables|Default|SetCueTarget (Variables|Default|GetMouseHitActor))
    (else
      (Variables|Default|SetCueTarget (Ability|GetAvatarActorfromActorInfo))))
  (GameplayCue|AddGameplayCueOnActor(Looping) (Variables|Default|GetCueTarget) "(TagName=\"GameplayCue.ShockLoop\")" (Variables|Default|GetFirstTargetCueParams))
  (if (Variables|Default|GetFirstTargetImplementsInterface)
    (bind _outadditionaltargets (Class|AuraBeemSpell|StoreAdditionalTarget))
    (bind _output_get_2 (Variables|Default|SetAdditional%20Targets _outadditionaltargets))
    (for _array_element _output_get_2
      (CallFunction|AddShockLoopCuetoAdditionalTargets _array_element))))

(fn AddShockLoopCuetoAdditionalTargets
  (params (AdditionalTarget :type Actor%20Object%20Reference))
  (bind _output_get (LocalVariables|SetTargetActor AdditionalTarget))
  (Utilities|Map|Add (Variables|Default|GetAdditionalActorsToCueParams) _output_get (Ability|GameplayCue|MakeGameplayCueParameters :Location (Transformation|GetActorLocation (LocalVariables|GetTargetActor)) :SourceObject (LocalVariables|GetTargetActor) :TargetAttachComponent (Variables|/Script/Engine.Actor|GetRootComponent (Variables|Default|GetMouseHitActor))))
  (GameplayCue|AddGameplayCueOnActor(Looping) (LocalVariables|GetTargetActor) "(TagName=\"GameplayCue.ShockLoop\")" (Ability|GameplayCue|MakeGameplayCueParameters :Location (Transformation|GetActorLocation (LocalVariables|GetTargetActor)) :SourceObject (LocalVariables|GetTargetActor) :TargetAttachComponent (Variables|/Script/Engine.Actor|GetRootComponent (Variables|Default|GetMouseHitActor)))))

(fn RemoveShockLoopfromAdditionalTargets
  (params (InputPin :type Actor%20Object%20Reference))
  (LocalVariables|SetAdditionalTargets InputPin)
  (if (.ReturnValue (Utilities|Map|Find (Variables|Default|GetAdditionalActorsToCueParams) (LocalVariables|GetAdditionalTargets)))
    (GameplayCue|RemoveGameplayCueOnActor(Looping) (LocalVariables|GetAdditionalTargets) "(TagName=\"GameplayCue.ShockLoop\")" (.Value (Utilities|Map|Find (Variables|Default|GetAdditionalActorsToCueParams) (LocalVariables|GetAdditionalTargets))))))