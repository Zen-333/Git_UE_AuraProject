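; Fire Blast fireball projectile that flies out and returns like a boomerang, then explodes.
; On the server, one timeline lerps it forward to an apex, then a second homes it back to the moving ReturnToActor.
; Within explode distance, it triggers OnHit, applies radial damage through Ability System effect params to nearby live players except its owner, then destroys itself.
; Knockback points away from the blast with pitch overridden to 45 degrees.
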(event EventStartOutgoingTimeline
  (bind _returnvalue (Components|GetOwner))
  (bind _self self)
  (bind _explosiondamageparams (Variables|Default|GetExplosionDamageParams))
  (bind _array (Utilities|Array|MakeArray _returnvalue))
  (Networking|SwitchHasAuthority
    (:Authority
      (Variables|Default|SetInitialLocation (Transformation|GetActorLocation))
      (Variables|Default|SetApexLocation (+ (Variables|Default|GetInitialLocation) (* (Transformation|GetActorForwardVector) (Variables|Default|GetTravelDistance))))
      (bind _outgoingtrack (Timeline|OutgoingTimeline Play)
        (:Update
          (Transformation|SetActorLocation (Math|Vector|Lerp(Vector) (Variables|Default|GetInitialLocation) (Variables|Default|GetApexLocation) _outgoingtrack) false false))
        (:Finished
          (bind _returningtrack (Timeline|ReturningTimeline Play)
            (:Update
              (Transformation|SetActorLocation (Math|Vector|Lerp(Vector) (Variables|Default|GetApexLocation) (Transformation|GetActorLocation (Variables|Default|GetReturnToActor)) _returningtrack) false false)
              (if (CallFunction|IsWithinExplodeDistance)
                (Class|AuraProjectile|OnHit)
                (Utilities|Array|Add _array _self)
                (bind _outoverlapingactors (Class|AuraAbilitySystemLibrary|GetLivePlayerWithinRadius _self _array 3e+02 (Transformation|GetActorLocation)))
                (bind _output_get (Variables|Default|SetOverlappingPlayers _outoverlapingactors))
                (Class|AuraAbilitySystemLibrary|SetIsRadialDamageEffectParam (Variables|Default|GetExplosionDamageParams) true 5e+01 3e+02 (Transformation|GetActorLocation))
                (for _array_element _output_get
                  (Class|AuraAbilitySystemLibrary|SetTargetEffectParamsASC (Variables|Default|GetExplosionDamageParams) (Ability|GetAbilitySystemComponent _array_element))
                  (Variables|Default|SetKnockbackDirection (- (Transformation|GetActorLocation _array_element) (Transformation|GetActorLocation)))
                  (Class|AuraAbilitySystemLibrary|SetKnockbackDirection (Variables|Default|GetExplosionDamageParams) (CallFunction|OverideKnockbackPitch) 8e+02)
                  (Class|AuraAbilitySystemLibrary|SetDeathImpulseDirection _explosiondamageparams (- (Transformation|GetActorLocation _array_element) (Transformation|GetActorLocation)) 6e+02)
                  (Class|AuraAbilitySystemLibrary|ApplyDamageEffect _explosiondamageparams))
                (Actor|DestroyActor)))))))))

(fn ConstructionScript)

(fn IsWithinExplodeDistance
  (return (<= (Math|Vector|VectorLength (- (Transformation|GetActorLocation) (Transformation|GetActorLocation (Variables|Default|GetReturnToActor)))) (Variables|Default|GetExplodeDistance))))

(fn OverideKnockbackPitch
  (bind _knockbackdirection (Variables|Default|GetKnockbackDirection))
  (bind _returnvalue (Math|Rotator|MakeRotfromX _knockbackdirection))
  (return (Math|Vector|GetForwardVector (Math|Rotator|MakeRotator (.roll _returnvalue) 45.0 (.yaw _returnvalue)))))