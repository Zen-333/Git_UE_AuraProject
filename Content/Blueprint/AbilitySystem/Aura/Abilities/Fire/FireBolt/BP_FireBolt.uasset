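; BP_FireBolt is the Fire Bolt projectile actor for the Aura fire ability.
; Shortly after BeginPlay it switches its Sphere to query-only collision.
; Each Tick it compares its location with the previous frame's and, if it moved no more than MinDistancePerFrame, spawns the impact sound and Niagara explosion, then destroys itself.
; This stall check applies no damage itself.
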(event EventBeginPlay
  (bind _sphere (Variables|Default|GetSphere))
  (Utilities|FlowControl|Delay 0.1)
  (Utilities|IsValid _sphere
    (:Is%20Valid
      (Collision|SetCollisionEnabled _sphere "QueryOnly"))))

(event Collision|EventActorBeginOverlap
  (params (OtherActor :type Actor%20Object%20Reference)))

(event EventTick
  (params (DeltaSeconds :type Float%20%28single-precision%29))
  (CallFunction|MakeGoKaboomifNoMove))

(fn ConstructionScript)

(fn MakeGoKaboomifNoMove
  (Variables|Default|SetLocationLastFrame (Variables|Default|GetLocationThisFram))
  (Variables|Default|SetLocationThisFram (Transformation|GetActorLocation))
  (if (<= (Math|Vector|VectorLength (- (Variables|Default|GetLocationThisFram) (Variables|Default|GetLocationLastFrame))) (Variables|Default|GetMinDistancePerFrame))
    (Audio|SpawnSoundatLocation "/Game/Assets/Sounds/Abilities/FireBolt/sfx_FireBolt_Impact.sfx_FireBolt_Impact" (Variables|Default|GetLocationThisFram) "0, 0, 0" 1.0 1.0 0.0 0 0)
    (Niagara|SpawnSystematLocation "/Game/Assets/Effects/Projectiles/FireExplosion/NS_FireExplosion1.NS_FireExplosion1" (Variables|Default|GetLocationThisFram))
    (Actor|DestroyActor)))