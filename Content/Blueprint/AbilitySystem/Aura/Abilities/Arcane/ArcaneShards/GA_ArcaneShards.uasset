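; Arcane Shards gameplay ability: shows a magic circle, waits for an input press, then erupts shards around the targeted ground point.
; A spawned BP_PointCollection supplies randomly rotated ground points, their count set by ability level up to a cap.
; After the cast montage's gameplay event, a looping timer fires one shard per point, applying radial damage with outward knockback and a gameplay cue.
; Cost commits when shards start; cooldown commits when they finish.
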(event Custom|SpawnShards
  (if (< (Variables|Default|GetCount) (Variables|Default|GetNumShards))
    (CallFunction|StoreShardsLocation)
    (CallFunction|StorePlayerstoDamage)
    (for _array_element (Variables|Default|GetPlayersToDamage)
      (CallFunction|RadialDamagetoPlayer _array_element))
    (Math|Integer|IncrementInt (Variables|Default|GetCount)
      (:%20%20
        (Class|GameplayAbility|ExecuteGameplayCuewithParams "(TagName=\"GameplayCue.ArcaneShards\")" (Ability|GameplayCue|MakeGameplayCueParameters :Location (Variables|Default|GetShardsSpawnLocation)))))
    (else
      (Utilities|Time|ClearandInvalidateTimerbyHandle (Variables|Default|GetShardsSpawnTimer))
      (Actor|DestroyActor (Variables|Default|GetPointCollection))
      (Ability|CommitAbilityCooldown false)
      (Ability|EndAbility))))

(event Ability|EventActivateAbility
  (bind _returnvalue (Class|GameplayAbility|CheckAbilityCost))
  (if _returnvalue
    (Utilities|FlowControl|Sequence
      (:then_0
        (Class|PlayerInterface|ShowMagicCircle(Message) (Ability|GetAvatarActorfromActorInfo) 0))
      (:then_1
        (Ability|Tasks|WaitInputPress false
          (:OnPress
            (bind _datahandle (|TargetDataUnderMouse)
              (:ValidData
                (Variables|Default|SetMouseHitLocation (.ImpactPoint (Collision|BreakHitResult (Ability|TargetData|GetHitResultfromTargetData _datahandle))))
                (bind _returnvalue_2 (Game|SpawnActorfromClass "/Game/Blueprint/AbilitySystem/Aura/Abilities/Arcane/ArcaneShards/BP_PointCollection.BP_PointCollection_C" (Math|Transform|MakeTransform (.ImpactPoint (Collision|BreakHitResult (Ability|TargetData|GetHitResultfromTargetData _datahandle))) "0, 0, 0" "1.000000,1.000000,1.000000") "AlwaysSpawn" "MultiplyWithRoot" 0 0))
                (bind _output_get (Variables|Default|SetPointCollection _returnvalue_2))
                (Variables|Default|SetNumShards (Math|Integer|Min(Integer) (Variables|Default|GetMaxNumShards) (Ability|GetAbilityLevel)))
                (Variables|Default|SetGroundPoints (Class|PointCollection|GetGroundPoints _output_get (Variables|Default|GetMouseHitLocation) (Variables|Default|GetNumShards) (Math|Random|RandomFloatinRange 0.0 3.6e+02)))
                (Class|CombatInterface|UpdateFacingTarget(Message) (Ability|GetAvatarActorfromActorInfo) (Variables|Default|GetMouseHitLocation))
                (|PlayMontageandWaitProxy "None" "/Game/Assets/Characters/Aura/Animations/Abilities/AN_CastArcaneShards.AN_CastArcaneShards" 1.0 "None" false 1.0 0.0
                  (:then
                    (Ability|Tasks|WaitGameplayEvent "(TagName=\"Event.Montage.ArcaneShards\")" 0 true
                      (:EventReceived
                        (bind _returnvalue_3 (Utilities|Time|SetTimerbyEvent (delegate Custom|SpawnShards) (Variables|Default|GetShardsSpawnDeltaTime) true))
                        (Variables|Default|SetShardsSpawnTimer _returnvalue_3)
                        (CallFunction|SpawnShards)
                        (Ability|CommitAbilityCost false)
                        (Class|PlayerInterface|HideMagicCircle(Message) (Ability|GetAvatarActorfromActorInfo))))))))))))))

(event Ability|EventOnEndAbility
  (params (bWasCancelled :type Boolean)))

(fn StoreShardsLocation
  (Variables|Default|SetShardsSpawnLocation (Transformation|GetWorldLocation (Utilities|Array|Get(acopy) (Variables|Default|GetGroundPoints) (Variables|Default|GetCount)))))

(fn StorePlayerstoDamage
  (bind _returnvalue (Ability|GetAvatarActorfromActorInfo))
  (bind _outoverlapingactors (Class|AuraAbilitySystemLibrary|GetLivePlayerWithinRadius _returnvalue (Utilities|Array|MakeArray _returnvalue) (Variables|Default|GetRadialDamageOuterRadius) (Variables|Default|GetShardsSpawnLocation)))
  (Variables|Default|SetPlayersToDamage _outoverlapingactors))

(fn RadialDamagetoPlayer
  (params (TargetActor :type Actor%20Object%20Reference))
  (bind _returnvalue (Transformation|GetActorLocation TargetActor))
  (bind _shardsspawnlocation (Variables|Default|GetShardsSpawnLocation))
  (bind _returnvalue_2 (- _returnvalue _shardsspawnlocation))
  (Class|AuraAbilitySystemLibrary|ApplyDamageEffect (Class|AuraDamageGameplayAbility|MakeDamageEffectParamsfromClassDefaults TargetActor (Variables|Default|GetShardsSpawnLocation) true _returnvalue_2 false _returnvalue_2 true 35.0)))